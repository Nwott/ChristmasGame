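; BP_House1 is a destructible house built on a Chaos Geometry Collection that collapses when hit.
; The Construction Script adds the anchor field child actor to the collection's initialization fields.
; A component hit removes all anchors and applies a kinematic field at the collection's location to free the pieces.
; A Chaos break event destroys the collection component after a short delay, clearing the debris.
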(event `self.SM_House_01_GeometryCollection.OnComponentHit`
  (params (HitComponent :type "PrimitiveComponent Object Reference") (OtherActor :type "Actor Object Reference") (OtherComp :type "PrimitiveComponent Object Reference") (NormalImpulse :type "Vector Structure") (Hit :type "HitResult Structure (by ref)"))
  (bind _sm_house_01_geometrycollection (`self.SM_House_01_GeometryCollection`))
  (`GeometryCollectionComponent.RemoveAllAnchors` _sm_house_01_geometrycollection)
  (`GeometryCollectionComponent.ApplyKinematicField` _sm_house_01_geometrycollection 500.0 (`SceneComponent.K2_GetComponentLocation` _sm_house_01_geometrycollection)))

(event `self.SM_House_01_GeometryCollection.OnChaosBreakEvent`
  (params (BreakEvent :type "ChaosBreakEvent Structure (by ref)"))
  (`KismetSystemLibrary.Delay` 5.0)
  (`ActorComponent.K2_DestroyComponent` (`self.SM_House_01_GeometryCollection`)))

(fn `UserConstructionScript`
  (`parent.UserConstructionScript`)
  (bind _asfs_anchor_field_generic (cast `/Engine/EditorResources/FieldNodes/FS_AnchorField_Generic` (`ChildActorComponent.ChildActor` (`self.FS_AnchorField_Generic`))))
  (`KismetArrayLibrary.Array_Add` (`GeometryCollectionComponent.InitializationFields` (`self.SM_House_01_GeometryCollection`)) _asfs_anchor_field_generic))